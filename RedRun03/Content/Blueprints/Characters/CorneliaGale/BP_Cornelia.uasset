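; BP_Cornelia is a side-scrolling PaperZD player character with movement, jump, dash and wall-slide detection.
; Enhanced Input drives X-axis movement, with control rotation flipping by acceleration to track facing.
; Dash launches along that facing behind a DoOnce, changing gravity when airborne until a delay ends.
; Hitting a "Wall"-tagged actor while falling plays the wall animation and holds a Wallslide flag through a retriggerable delay.
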(event Input|EnhancedActionEvents|EnhancedInputActionIA_Dash
  (params (ActionValue :type Boolean) (ElapsedSeconds :type Float%20%28double-precision%29) (TriggeredSeconds :type Float%20%28double-precision%29) (InputAction :type Input%20Action%20Object%20Reference :default "/Game/Input/Actions/IA_Dash.IA_Dash"))
  (bind _launchspeed (Variables|Default|GetLaunchSpeed))
  (bind _charactermovement (Variables|Character|GetCharacterMovement))
  (Utilities|FlowControl|DoOnce false :!label _label
    (:Completed
      (Class|PaperZDAnimInstance|JumptoNode (Variables|/Script/PaperZD.PaperZDAnimationComponent|GetAnimInstance (Variables|Default|GetPaperZDAnimation)) "Dash" "None")
      (if (AI|Components|NavMovement|IsFalling _charactermovement)
        (Variables|/Script/Engine.CharacterMovementComponent|SetGravityScale _charactermovement (Variables|Default|GetDashingGravity)))
      (Character|LaunchCharacter (Math|Vector|MakeVector (select (Variables|Default|GetMovingRight) _launchspeed (* _launchspeed -1.0)) 0.0 0.0) true true)
      (Variables|Default|SetisDashing true)
      (Utilities|FlowControl|Delay (Variables|Default|GetDashDuration))
      (Variables|Default|SetisDashing false)
      (Variables|/Script/Engine.CharacterMovementComponent|SetGravityScale (Variables|Character|GetCharacterMovement) (Variables|Default|GetDefaultGravity))
      (goto _label Reset))))

(event Input|EnhancedActionEvents|EnhancedInputActionIA_Jump
  (params (ActionValue :type Boolean) (ElapsedSeconds :type Float%20%28double-precision%29) (TriggeredSeconds :type Float%20%28double-precision%29) (InputAction :type Input%20Action%20Object%20Reference :default "/Game/Input/Actions/IA_Jump.IA_Jump"))
  (:Started
    (Character|Jump)))

(event Input|EnhancedActionEvents|EnhancedInputActionIA_Move
  (params (ActionValue :type Vector%202D%20Structure) (ElapsedSeconds :type Float%20%28double-precision%29) (TriggeredSeconds :type Float%20%28double-precision%29) (InputAction :type Input%20Action%20Object%20Reference :default "/Game/Input/Actions/IA_Move.IA_Move"))
  (CallFunction|RotateComtroller)
  (Pawn|Input|AddMovementInput "1.000000,0.000000,0.000000" (Math|Conversions|ToFloat(Integer) (Math|Float|Round (.x ActionValue))) false))

(event EventBeginPlay
  (bind _asplayer_controller (Utilities|Casting|CastToPlayerController (Pawn|GetController)))
  (Input|AddMappingContext (PlayerController|LocalPlayerSubsystems|GetEnhancedInputLocalPlayerSubsystem _asplayer_controller) "/Game/Input/IMC_RedRun.IMC_RedRun" 0 "(bIgnoreAllPressedKeysUntilRelease=True,bForceImmediately=False,bNotifyUserSettings=False)"))

(event Collision|EventHit
  (params (MyComp :type Primitive%20Component%20Object%20Reference) (Other :type Actor%20Object%20Reference) (OtherComp :type Primitive%20Component%20Object%20Reference) (bSelfMoved :type Boolean) (HitLocation :type Vector :default "0, 0, 0") (HitNormal :type Vector :default "0, 0, 0") (NormalImpulse :type Vector :default "0, 0, 0") (Hit :type Hit%20Result%20Structure%20%28by%20ref%29))
  (if (and (Actor|ActorHasTag Other "Wall") (AI|Components|NavMovement|IsFalling (Variables|Character|GetCharacterMovement)))
    (Variables|Default|SetWallslide true)
    (Class|PaperZDAnimInstance|JumptoNode (Variables|/Script/PaperZD.PaperZDAnimationComponent|GetAnimInstance (Variables|Default|GetPaperZDAnimation)) "OnAWall" "None")
    (Utilities|FlowControl|RetriggerableDelay 0.1)
    (Variables|Default|SetWallslide false)))

(fn ConstructionScript)

(fn RotateComtroller
  (Math|Float|CompareFloat (.x (Pawn|Components|CharacterMovement|GetCurrentAcceleration (Variables|Character|GetCharacterMovement))) 0.0
    (:>
      (Pawn|SetControlRotation (Pawn|GetController) (Math|Rotator|MakeRotator 0.0 0.0 0.0))
      (Variables|Default|SetMovingRight true))
    (:<
      (Pawn|SetControlRotation (Pawn|GetController) (Math|Rotator|MakeRotator 0.0 0.0 1.8e+02))
      (Variables|Default|SetMovingRight false))))