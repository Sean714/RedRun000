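; Parent Blueprint for dialog NPCs that the player (BP_Cornelia) can talk to.
; An overlap box toggles a prompt widget and registers or clears the NPC as the player's interactable.
; Interact sends the player the DialogList entry matching CurrentDialogID.
; SetDialogTarget changes that ID and continues unless End is set, while a GI_RedRun dispatcher retargets NPCs by name.
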(event OnComponentBeginOverlap(Box)
  (params (OverlappedComponent :type Primitive%20Component%20Object%20Reference) (OtherActor :type Actor%20Object%20Reference) (OtherComp :type Primitive%20Component%20Object%20Reference) (OtherBodyIndex :type Integer) (bFromSweep :type Boolean) (SweepResult :type Hit%20Result%20Structure%20%28by%20ref%29))
  (bind _player (Variables|Default|GetPlayer))
  ;[0 1 0 0] Begin Overlap Interact Logic - set Interactor
  (if (== OtherActor _player)
    (Rendering|SetVisibility (Variables|Default|GetWidget) true false)
    (Class|BPIInteract|SetInteractableActor(Message) _player self)))

(event OnComponentEndOverlap(Box)
  (params (OverlappedComponent :type Primitive%20Component%20Object%20Reference) (OtherActor :type Actor%20Object%20Reference) (OtherComp :type Primitive%20Component%20Object%20Reference) (OtherBodyIndex :type Integer))
  (bind _player (Variables|Default|GetPlayer))
  ;[0 1 0 0] End Overlap Interact logic - clear Interactor.
  (if (== OtherActor _player)
    (Rendering|SetVisibility (Variables|Default|GetWidget) false false)
    (Class|BPIInteract|SetInteractableActor(Message) _player)))

(event Custom|ReceiveSetDialogDispatch
  (params (Name :type Name) (DialogTarget :type Integer))
  ;[0 1 0 0] Set New Dialog Target from Quest Manager
  (if (== Name (Variables|Default|GetMyName))
    (Variables|Default|SetCurrentDialogID DialogTarget)))

(event EventBeginPlay
  ;[0 1 0 0] Get Game Instance variable, Bind Set Dialog Listener, Get Player Reference.
  (bind _output_get (Variables|Default|SetGameInstance (Game|GetGameInstance)))
  (bind _asgi_red_run (Utilities|Casting|CastToGI_RedRun _output_get))
  (EventDispatchers|BindEventtoDispatchSetDialog _asgi_red_run (delegate Custom|ReceiveSetDialogDispatch))
  (bind _asbp_cornelia (Utilities|Casting|CastToBP_Cornelia (Game|GetPlayerCharacter 0)))
  (Variables|Default|SetPlayer _asbp_cornelia))

(event EventInteract
  ;[0 1 0 0] Interact - Send Dialog
  (Rendering|SetVisibility (Variables|Default|GetWidget) false false)
  (for (_array_element _array_index) (Variables|Default|GetDialogList)
    (if (== (.id _array_element) (Variables|Default|GetCurrentDialogID))
      (Default|SendDialog (Variables|Default|GetPlayer) (Utilities|Array|Get(acopy) (Variables|Default|GetDialogList) _array_index)))))

(event EventSetDialogTarget
  (params (DialogTarget :type Integer) (End :type Boolean))
  ;[0 1 0 0] Set New Dialog ID. Send back to Player or end.
  (Variables|Default|SetCurrentDialogID DialogTarget)
  (if (not End)
    (CallFunction|Interact)))

(fn ConstructionScript)