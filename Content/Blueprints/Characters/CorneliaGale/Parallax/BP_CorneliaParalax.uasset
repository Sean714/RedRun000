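; BP_CorneliaParalax is a parallax background actor built from Paper2D sprites, kept with the Cornelia Gale character assets.
; On BeginPlay it gives each sprite under StaticBackground a dynamic material instance, stores it in DynamicLayers and sets its ParallaxMultiplier from a per-layer array matched by child index.
; Backgroundon and BackgroundOff events show or hide all those sprites and print debug messages.
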(event EventBeginPlay
  (|CallParentFunction)
  (CallFunction|CollectParallaxLayers))

(event EventBackgroundon
  (Development|PrintString "On!!!" true true "(R=0.000000,G=0.660000,B=1.000000,A=1.000000)" 1e+01)
  (for _array_element (Components|GetChildrenComponents (Variables|Default|GetStaticBackground) false)
    (bind _aspaper_sprite_component (Utilities|Casting|CastToPaperSpriteComponent _array_element))
    (Rendering|SetVisibility _aspaper_sprite_component true false)))

(event EventBackgroundOff
  (Development|PrintString "Off!!" true true "(R=0.000000,G=0.660000,B=1.000000,A=1.000000)" 1e+01)
  (for _array_element (Components|GetChildrenComponents (Variables|Default|GetStaticBackground) false)
    (bind _aspaper_sprite_component (Utilities|Casting|CastToPaperSpriteComponent _array_element))
    (Rendering|SetVisibility _aspaper_sprite_component false false)))

(fn ConstructionScript
  (|CallParentFunction))

(fn CollectParallaxLayers
  (for (_array_element _array_index) (Components|GetChildrenComponents (Variables|Default|GetStaticBackground) false)
    (bind _aspaper_sprite_component (Utilities|Casting|CastToPaperSpriteComponent _array_element))
    (bind _returnvalue (Rendering|Material|CreateDynamicMaterialInstance _aspaper_sprite_component 0 0 "None" :!class /Script/Engine.PrimitiveComponent))
    (Utilities|Array|Add (Variables|Default|GetDynamicLayers) _returnvalue)
    (Rendering|Material|SetScalarParameterValue _returnvalue "ParallaxMultiplier" (Utilities|Array|Get(acopy) (Variables|Default|GetParallaxMultiplier) _array_index) :!class /Script/Engine.MaterialInstanceDynamic)))