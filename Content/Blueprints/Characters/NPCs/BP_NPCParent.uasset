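; BP_NPCParent is the base NPC Blueprint that gives the player character dialog matching the NPC's current dialog ID.
; On BeginPlay it binds to the GI_RedRun game instance's set-dialog dispatcher and caches the BP_Cornelia player.
; Dispatches matching its name update that ID, letting quest logic switch dialog.
; Interact searches the dialog list for that ID and sends matching entries to the player.
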(event Custom|ReceiveSetDialogDispatch
  (params (Name :type Name) (DialogTarget :type Integer))
  (bind _myname (Variables|Default|GetMyName))
  ;[0 1 0] Set New Dialog Target from QUest Manager
  (Development|PrintString "Received Dispatch!")
  (if (== Name _myname)
    (Variables|Default|SetCurrentDialogID DialogTarget)
    (Development|PrintString (Utilities|String|Append "New Dialog Target set for: " (Utilities|String|ToString(Name) _myname)))))

(event EventBeginPlay
  (bind _output_get (Variables|Default|SetGameInstance (Game|GetGameInstance)))
  (bind _asgi_red_run (Utilities|Casting|CastToGI_RedRun _output_get))
  (EventDispatchers|BindEventtoDispatchSetDialog _asgi_red_run (delegate Custom|ReceiveSetDialogDispatch))
  (bind _asbp_cornelia (Utilities|Casting|CastToBP_Cornelia (Game|GetPlayerCharacter 0)))
  (Variables|Default|SetPlayer _asbp_cornelia))

(event Collision|EventActorBeginOverlap
  (params (OtherActor :type Actor%20Object%20Reference)))

(event EventTick
  (params (DeltaSeconds :type Float%20%28single-precision%29)))

(event EventInteract
  (for (_array_element _array_index) (Variables|Default|GetDialogList)
    (if (== (.id _array_element) (Variables|Default|GetCurrentDialogID))
      (Default|SendDialog (Variables|Default|GetPlayer) (Utilities|Array|Get(acopy) (Variables|Default|GetDialogList) _array_index)))))

(fn ConstructionScript)