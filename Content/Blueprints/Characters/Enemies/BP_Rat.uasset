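; BP_Rat is a rat enemy character Blueprint with a placeholder melee or proximity attack check.
; The Attafck function compares its distance to the Player against AttackDistance and, when within range, only prints an "Attack!" debug message.
; The construction script just calls the parent, and nothing shown here invokes the attack function or applies damage.
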(fn ConstructionScript
  (|CallParentFunction))

(fn Attafck
  (if (< (Math|Vector|Distance(Vector) (Transformation|GetActorLocation (Variables|Default|GetPlayer)) (Transformation|GetActorLocation self)) (Variables|Default|GetAttackDistance))
    (Development|PrintString "Attack!" true true "(R=0.000000,G=0.660000,B=1.000000,A=1.000000)" 2e+01)))