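; Base enemy Blueprint that walks forward continuously until stopped and reverses its facing on ChangeDirection while not aggroed.
; Aggro runs once, starting looping timers that re-orient it using the cached BP_Cornelia player's location, constrained to the X axis, and periodically call Attack.
; Ranged enemies stop moving when aggroed, and Attack is an empty function in this base.
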(event Custom|LookAtLoop
  (Transformation|SetActorRotation (Math|Conversions|RotationFromXVector (Math|Vector|MakeVector (.roll (Math|Rotator|FindLookatRotation (Transformation|GetActorLocation) (Transformation|GetActorLocation (Variables|Default|GetPlayer)))) 0.0 0.0))))

(event Custom|AttackLoop
  (CallFunction|Attack))

(event EventBeginPlay
  (bind _asbp_cornelia (Utilities|Casting|CastToBP_Cornelia (Game|GetPlayerCharacter 0)))
  (Variables|Default|SetPlayer _asbp_cornelia))

(event EventTick
  (params (DeltaSeconds :type Float%20%28single-precision%29))
  (if (not (Variables|Default|GetisStopped))
    (Pawn|Input|AddMovementInput (Transformation|GetActorForwardVector) 1.0 false)))

(event EventChangeDirection
  (if (not (Variables|Default|GetisAggro))
    (CallFunction|ChangeMyDirection)))

(event EventAggro
  (if (not (Variables|Default|GetisAggro))
    (Variables|Default|SetisAggro true)
    (bind _returnvalue (Utilities|Time|SetTimerbyEvent (delegate Custom|LookAtLoop) 0.1 true))
    (Variables|Default|SetLookTimerHandle _returnvalue)
    (bind _returnvalue_2 (Utilities|Time|SetTimerbyEvent (delegate Custom|AttackLoop) 2.0 true))
    (Variables|Default|SetAttackTimerHandle _returnvalue_2)
    (if (Variables|Default|GetisRanged)
      (Variables|Default|SetisStopped true))))

(fn ConstructionScript)

(fn ChangeMyDirection
  (Transformation|SetActorRotation (Math|Rotator|CombineRotators (Transformation|GetActorRotation) "0.000000,180.000000,0.000000")))

(fn Attack)