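; GL_RedRun holds the game's quest list, with an unfinished function for starting quests.
; On Init it copies every DT_QuestList row into QuestList, printing each name.
; StartQuestFunc calls SearchQuestList to look up an ID, but its branch does nothing and its return and array-update nodes are unwired.
; SearchQuestList returns after checking only the first element, and reports the input ID as FoundID even without a match.
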(event EventInit
  ;[0 1 0] Read quest table into QuestList
  (bind _outrownames (DataTable|GetDataTableRowNames "/Game/Data/DT_QuestList.DT_QuestList"))
  (for _array_element _outrownames
    (bind _returnvalue (Utilities|GetDataTableRow "/Game/Data/DT_QuestList.DT_QuestList" _array_element)
      (:then
        (Utilities|Array|Add (Variables|Default|GetQuestList) _returnvalue)
        (Development|PrintString (Utilities|String|Append "Added!!" (Utilities|String|ToString(Text) (.Name (Utilities|Struct|BreakFQuests _returnvalue)))))))))

(fn StartQuestFunc
  (params (QuestID :type Integer))
  ;[0.15 0.15 0.15 0.5] Comment
  (bind _foundid (CallFunction|SearchQuestList QuestID))
  (if (== _foundid -1)
    _))

(fn SearchQuestList
  (params (InputID :type Integer))
  (for (_array_element _array_index) (Variables|Default|GetQuestList)
    (if (== (.id _array_element) InputID)
      (Development|PrintString "QuestFound!!" true true "(R=0.000000,G=0.660000,B=1.000000,A=1.000000)" 5.0)
      (return InputID _array_index)
      (else
        (Development|PrintString "Quest Not Found!!" true true "(R=0.000000,G=0.660000,B=1.000000,A=1.000000)" 5.0)
        (return InputID -1)))))