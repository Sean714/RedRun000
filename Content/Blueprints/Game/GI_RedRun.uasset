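; Game Instance for RedRun that holds the quest list and exposes functions to start, end and query quests.
; On Init it copies DT_QuestList rows into QuestList.
; Quest functions use SearchQuestList, which returns after checking only the first entry, and start or end quests by rewriting the record with a new Status.
; The end-target loop for NPC dialog is empty, and the SetDialog dispatcher calls are unconnected.
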(event EventInit
  ;[0 1 0] Read quest table into QuestList
  (bind _outrownames (DataTable|GetDataTableRowNames "/Game/Data/DT_QuestList.DT_QuestList"))
  (for _array_element _outrownames
    (bind _returnvalue (Utilities|GetDataTableRow "/Game/Data/DT_QuestList.DT_QuestList" _array_element)
      (:then
        (Utilities|Array|Add (Variables|Default|GetQuestList) _returnvalue)
        (Development|PrintString (Utilities|String|Append "Added!!" (Utilities|String|ToString(Text) (.Name (Utilities|Struct|BreakFQuests _returnvalue)))))))))

(fn SearchQuestList
  (params (InputID :type Integer))
  (for (_array_element _array_index) (Variables|Default|GetQuestList)
    (if (== (.id _array_element) InputID)
      (Development|PrintString "QuestFound!!" true true "(R=0.000000,G=0.660000,B=1.000000,A=1.000000)" 5.0)
      (return InputID _array_index)
      (else
        (Development|PrintString "Quest Not Found!!" true true "(R=0.000000,G=0.660000,B=1.000000,A=1.000000)" 5.0)
        (return InputID -1)))))

(fn EndQuest
  (params (QuestID :type Integer))
  ;[0 1 0] Set Quest to completed
  (Development|PrintString "End QUEST!!")
  (bind (_foundid _index) (CallFunction|SearchQuestList QuestID))
  (if (!= _index -1)
    (Utilities|Array|SetArrayElem (Variables|Default|GetQuestList) _index (Utilities|Struct|MakeFQuests (.id (Utilities|Array|Get(acopy) (Variables|Default|GetQuestList) _foundid)) (.name (Utilities|Array|Get(acopy) (Variables|Default|GetQuestList) _foundid)) (.description (Utilities|Array|Get(acopy) (Variables|Default|GetQuestList) _foundid)) "NewEnumerator2" (.endtargets (Utilities|Array|Get(acopy) (Variables|Default|GetQuestList) _foundid))))
    ;[0 1 0] SetNPCDialog - loop End Targets
    (for _array_element (.endtargets (Utilities|Array|Get(acopy) (Variables|Default|GetQuestList) _foundid))
      _)
    (return true)
    (else
      (return false))))

(fn GetQuest
  (params (QuestID :type Integer))
  ;[0 1 0] Search then return a Quest record.
  (bind (_foundid _index) (CallFunction|SearchQuestList QuestID))
  (if (!= _index -1)
    (return (Utilities|Array|Get(acopy) (Variables|Default|GetQuestList) _foundid) true)
    (else
      (return "" false))))

(fn GetQuestList
  (return (Variables|Default|GetQuestList)))

(fn GetQuestStatus
  (params (QuestID :type Integer))
  (bind (_foundid _index) (CallFunction|SearchQuestList))
  (if (!= _index -1)
    (return (.status (Utilities|Array|Get(acopy) (Variables|Default|GetQuestList) _foundid)) true)
    (else
      (return "NewEnumerator0" false))))

(fn StartQuest
  (params (QuestID :type Integer))
  (Development|PrintString "QUest Started!!! Called!" true true "(R=0.000000,G=0.660000,B=1.000000,A=1.000000)" 1e+01)
  (bind _index (CallFunction|SearchQuestList QuestID))
  (if (!= _index -1)
    (Utilities|Array|SetArrayElem (Variables|Default|GetQuestList) _index (Utilities|Struct|MakeFQuests (.id (Utilities|Array|Get(acopy) (Variables|Default|GetQuestList) _index)) (.name (Utilities|Array|Get(acopy) (Variables|Default|GetQuestList) _index)) (.description (Utilities|Array|Get(acopy) (Variables|Default|GetQuestList) _index)) "NewEnumerator1" (.endtargets (Utilities|Array|Get(acopy) (Variables|Default|GetQuestList) _index))))
    (Development|PrintString (Utilities|String|Append "Set Quest: " (Utilities|String|ToString(Text) (.name (Utilities|Array|Get(acopy) (Variables|Default|GetQuestList) _index))) " to started!!") true true "(R=0.000000,G=0.660000,B=1.000000,A=1.000000)" 2e+01)
    (return true)))