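; Locked door actor that BP_Rocky can open only when carrying a key that references it.
; Its sphere overlap registers the door as the other actor's interactable and toggles a prompt widget.
; Interact searches Rocky's KeyArray for a matching DoorRef, then plays an unlock sound and a timeline that yaws the root, or a fail sound.
; The yaw Lerp takes the timeline value as A, with Alpha fixed at 90.
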(event OnComponentBeginOverlap(Sphere)
  (params (OverlappedComponent :type Primitive%20Component%20Object%20Reference) (OtherActor :type Actor%20Object%20Reference) (OtherComp :type Primitive%20Component%20Object%20Reference) (OtherBodyIndex :type Integer) (bFromSweep :type Boolean) (SweepResult :type Hit%20Result%20Structure%20%28by%20ref%29))
  (Class|BPIInteract|SetInteractable(Message) OtherActor self)
  (Rendering|SetVisibility (Variables|Default|GetWidget) true false))

(event OnComponentEndOverlap(Sphere)
  (params (OverlappedComponent :type Primitive%20Component%20Object%20Reference) (OtherActor :type Actor%20Object%20Reference) (OtherComp :type Primitive%20Component%20Object%20Reference) (OtherBodyIndex :type Integer))
  (bind _interactableactor (Class|BPIInteract|GetInteractable(Message) OtherActor))
  (if (== _interactableactor self)
    (Class|BPIInteract|SetInteractable(Message) OtherActor)
    (Rendering|SetVisibility (Variables|Default|GetWidget) false false)))

(event EventBeginPlay)

(event EventInteract
  (params (Interactor :type Actor%20Object%20Reference))
  (bind _returnvalue (Transformation|GetActorLocation))
  (bind _asbp_rocky (Utilities|Casting|CastToBP_Rocky Interactor))
  (for _array_element (Variables|/Game/Blueprints/Character/BP_Rocky.BP_Rocky_C|GetKeyArray _asbp_rocky)
    (if (== (.doorref _array_element) self)
      (Variables|Default|Setopen? true)))
  (if (Variables|Default|Getopen?)
    (Audio|PlaySoundatLocation "/Game/Assets/Sounds/Door/Unlock_WAV.Unlock_WAV" _returnvalue "0, 0, 0" 1.0 1.0 0.0 0 0 0 0)
    (bind _pivotdoor (Timeline|OpenDoor Play)
      (:Update
        (Transformation|SetRelativeRotation (Variables|Default|GetDefaultSceneRoot) (Math|Rotator|MakeRotator 0.0 0.0 (Math|Float|Lerp _pivotdoor 0.0 9e+01)) false false)))
    (else
      (Audio|PlaySoundatLocation "/Game/Assets/Sounds/Door/Fail_WAV.Fail_WAV" _returnvalue "0, 0, 0" 1.0 1.0 0.0 0 0 0 0))))

(fn ConstructionScript)

(fn GetInteractable
  (return 0))