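; BP_PatrolBox is a box volume that bounds the patrol of one assigned enemy and triggers its aggro.
; It caches the BP_Cornelia player character on BeginPlay.
; When the assigned enemy leaves the box, the box tells it to change direction.
; When the player enters, the box sends the enemy an aggro message and destroys itself, removing the patrol boundary.
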(event OnComponentEndOverlap(Box)
  (params (OverlappedComponent :type Primitive%20Component%20Object%20Reference) (OtherActor :type Actor%20Object%20Reference) (OtherComp :type Primitive%20Component%20Object%20Reference) (OtherBodyIndex :type Integer))
  ;[0 0 1 0] Turn NPC Around
  (if (== OtherActor (Variables|Default|GetAssignedEnemy))
    (Default|ChangeMyDirection (Variables|Default|GetAssignedEnemy))))

(event OnComponentBeginOverlap(Box)
  (params (OverlappedComponent :type Primitive%20Component%20Object%20Reference) (OtherActor :type Actor%20Object%20Reference) (OtherComp :type Primitive%20Component%20Object%20Reference) (OtherBodyIndex :type Integer) (bFromSweep :type Boolean) (SweepResult :type Hit%20Result%20Structure%20%28by%20ref%29))
  ;[0 0 1 0] Player Sends Aggro
  (if (== OtherActor (Variables|Default|GetPlayer))
    (Class|BPIEnemy|Aggro(Message) (Variables|Default|GetAssignedEnemy))
    (Actor|DestroyActor)))

(event EventBeginPlay
  ;[0 0 1 0] Get Player Reference
  (bind _asbp_cornelia (Utilities|Casting|CastToBP_Cornelia (Game|GetPlayerCharacter 0)))
  (Variables|Default|SetPlayer _asbp_cornelia))

(fn ConstructionScript)