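; BP_LevelEnd is a level-exit trigger actor that loads the next level when the player, BP_Cornelia, enters its sphere.
; BeginPlay caches the player character as BP_Cornelia.
; On sphere overlap with that player, it passes its BackgroundOn setting to the Game Instance through SetBackgroundVisibilityMessage, then opens the level named by LevelName.
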(event OnComponentBeginOverlap(Sphere)
  (params (OverlappedComponent :type Primitive%20Component%20Object%20Reference) (OtherActor :type Actor%20Object%20Reference) (OtherComp :type Primitive%20Component%20Object%20Reference) (OtherBodyIndex :type Integer) (bFromSweep :type Boolean) (SweepResult :type Hit%20Result%20Structure%20%28by%20ref%29))
  ;[1 1 0 0] Send Background Visibility to GI. Load New Level.
  (if (== OtherActor (Variables|Default|GetPlayer))
    (Class|BPIGameInstance|SetBackgroundVisibility(Message) (Game|GetGameInstance) (Variables|Default|GetBackgroundOn?))
    (Game|OpenLevel(byName) (Variables|Default|GetLevelName))))

(event EventBeginPlay
  ;[1 1 0 0] Get Reference to PLayer.
  (bind _asbp_cornelia (Utilities|Casting|CastToBP_Cornelia (Game|GetPlayerCharacter 0)))
  (Variables|Default|SetPlayer _asbp_cornelia))

(fn ConstructionScript)