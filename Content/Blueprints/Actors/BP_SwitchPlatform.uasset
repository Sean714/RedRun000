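; BP_SwitchPlatform is a platform actor that starts shuttling back and forth once it receives an Interact event.
; The PingPong timeline drives InterpLocation, which lerps the Platform component between the actor's location and the TargetLocation component's world position without sweeping.
; On each finish, the timeline direction selects MoveBack or MoveForward, so the motion loops indefinitely.
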(event Custom|MoveBack
  ;[1 0 0] Do Movement
  (bind (_direction _newtrack_0) (Timeline|PingPong ReverseFromEnd)
    (:Update
      (CallFunction|InterpLocation _newtrack_0))
    (:Finished
      (switch Utilities|FlowControl|Switch|SwitchonETimelineDirection _direction
        (:Forward
          (CallFunction|MoveBack))
        (:Backward
          (CallFunction|MoveForward))))))

(event Custom|MoveForward
  ;[1 0 0] Do Movement
  (bind (_direction _newtrack_0) (Timeline|PingPong Play)
    (:Update
      (CallFunction|InterpLocation _newtrack_0))
    (:Finished
      (switch Utilities|FlowControl|Switch|SwitchonETimelineDirection _direction
        (:Forward
          (CallFunction|MoveBack))
        (:Backward
          (CallFunction|MoveForward))))))

(event EventInteract
  ;[1 0 0] Receive Interact Command
  (Development|PrintString "Called!")
  (CallFunction|MoveForward))

(fn ConstructionScript)

(fn InterpLocation
  (params (Alpha :type Float%20%28double-precision%29))
  (Transformation|SetWorldLocation (Variables|Default|GetPlatform) (Math|Vector|Lerp(Vector) (Transformation|GetActorLocation) (Transformation|GetWorldLocation (Variables|Default|GetTargetLocation)) Alpha) false false))