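; BP_Switch is an interactable switch actor that triggers an action on an assigned InteractTarget.
; Its sphere overlap registers the switch as the overlapping actor's interactable and shows a prompt widget, clearing both on exit if it is still the registered one.
; Interact plays the flipbook animation for a fraction of a second, stops it, then sends InteractMessage to the target if valid.
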(event OnComponentBeginOverlap(Sphere)
  (params (OverlappedComponent :type Primitive%20Component%20Object%20Reference) (OtherActor :type Actor%20Object%20Reference) (OtherComp :type Primitive%20Component%20Object%20Reference) (OtherBodyIndex :type Integer) (bFromSweep :type Boolean) (SweepResult :type Hit%20Result%20Structure%20%28by%20ref%29))
  (Class|BPIInteract|SetInteractable(Message) OtherActor self)
  (Rendering|SetVisibility (Variables|Default|GetWidget) true false))

(event OnComponentEndOverlap(Sphere)
  (params (OverlappedComponent :type Primitive%20Component%20Object%20Reference) (OtherActor :type Actor%20Object%20Reference) (OtherComp :type Primitive%20Component%20Object%20Reference) (OtherBodyIndex :type Integer))
  (bind _interactableactor (Class|BPIInteract|GetInteractable(Message) OtherActor))
  (if (== _interactableactor self)
    (Class|BPIInteract|SetInteractable(Message) OtherActor)
    (Rendering|SetVisibility (Variables|Default|GetWidget) false false)))

(event EventInteract
  (params (Interactor :type Actor%20Object%20Reference))
  (Audio|Components|Audio|Play (Variables|Default|GetPaperFlipbook))
  (Utilities|FlowControl|Delay 0.3)
  (Audio|Components|Audio|Stop (Variables|Default|GetPaperFlipbook))
  (bind _interacttarget (Variables|Default|GetInteractTarget)
    (:then
      (Class|BPIInteract|Interact(Message) _interacttarget))
    (:else)))

(fn ConstructionScript)

(fn GetInteractable
  (return 0))