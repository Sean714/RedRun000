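; BP_Key is a collectible key actor that the player picks up by touching it.
; On BeginPlay it finds the BP_Rocky actor in the level and caches it as Player.
; When its Sphere is overlapped, it adds an FKey entry pairing itself with its Door to the player's KeyArray, then destroys itself.
; The overlap does not check which actor entered the sphere.
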(event OnComponentBeginOverlap(Sphere)
  (params (OverlappedComponent :type Primitive%20Component%20Object%20Reference) (OtherActor :type Actor%20Object%20Reference) (OtherComp :type Primitive%20Component%20Object%20Reference) (OtherBodyIndex :type Integer) (bFromSweep :type Boolean) (SweepResult :type Hit%20Result%20Structure%20%28by%20ref%29))
  (Utilities|Array|Add (Variables|/Game/Blueprints/RockyTemp/BP_Rocky.BP_Rocky_C|GetKeyArray (Variables|Default|GetPlayer)) (Utilities|Struct|MakeFKey self (Variables|Default|GetDoor)))
  (Actor|DestroyActor))

(event EventBeginPlay
  (bind _outactors (Actor|GetAllActorsOfClass "/Game/Blueprints/RockyTemp/BP_Rocky.BP_Rocky_C"))
  (for _array_element _outactors
    (Variables|Default|SetPlayer _array_element)))

(fn ConstructionScript)