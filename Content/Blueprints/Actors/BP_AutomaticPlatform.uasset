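; BP_AutomaticPlatform is a moving platform that travels back and forth on its own between the actor's location and a TargetLocation component.
; The PingPong timeline starts on BeginPlay and feeds its track into InterpLocation, which lerps the Platform component's world location without sweeping.
; Each time the timeline finishes, its direction selects MoveBack or MoveForward, so the motion loops endlessly.
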(event Custom|MoveBack
  (bind (_direction _newtrack_0) (Timeline|PingPong ReverseFromEnd)
    (:Update
      (CallFunction|InterpLocation _newtrack_0))
    (:Finished
      (switch Utilities|FlowControl|Switch|SwitchonETimelineDirection _direction
        (:Forward
          (CallFunction|MoveBack))
        (:Backward
          (CallFunction|MoveForward))))))

(event Custom|MoveForward
  (bind (_direction _newtrack_0) (Timeline|PingPong Play)
    (:Update
      (CallFunction|InterpLocation _newtrack_0))
    (:Finished
      (switch Utilities|FlowControl|Switch|SwitchonETimelineDirection _direction
        (:Forward
          (CallFunction|MoveBack))
        (:Backward
          (CallFunction|MoveForward))))))

(event EventBeginPlay
  (CallFunction|MoveForward))

(fn ConstructionScript)

(fn InterpLocation
  (params (Alpha :type Float%20%28double-precision%29))
  (Transformation|SetWorldLocation (Variables|Default|GetPlatform) (Math|Vector|Lerp(Vector) (Transformation|GetActorLocation) (Transformation|GetWorldLocation (Variables|Default|GetTargetLocation)) Alpha) false false))