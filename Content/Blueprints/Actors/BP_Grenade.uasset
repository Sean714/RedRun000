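; BP_Grenade is a grenade actor that lands near the player, BP_Cornelia, and checks for a proximity hit after a short fuse.
; On BeginPlay it moves itself to the player's location plus TargetOffset, with the X offset following facing and leading by velocity.
; After the delay, a player within DamageDistance only triggers a debug "Damage!!" print, with no damage applied.
; The actor destroys itself shortly afterwards.
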(event EventBeginPlay
  (bind _targetoffset (Variables|Default|GetTargetOffset))
  (bind _asbp_cornelia (Utilities|Casting|CastToBP_Cornelia (Game|GetPlayerCharacter 0)))
  (Transformation|SetActorLocation (+ (Transformation|GetActorLocation _asbp_cornelia) (Math|Vector|MakeVector (* (.x (Transformation|GetActorForwardVector _asbp_cornelia)) (+ (* (.x (Transformation|GetActorForwardVector _asbp_cornelia)) (.x (Transformation|GetVelocity _asbp_cornelia))) (.x _targetoffset))) (.y _targetoffset) (.z _targetoffset))) false false)
  (Utilities|FlowControl|Delay 1.5)
  (if (< (Transformation|GetDistanceTo _asbp_cornelia) (Variables|Default|GetDamageDistance))
    (Development|PrintString "Damage!!" true true "(R=0.000000,G=0.660000,B=1.000000,A=1.000000)" 5.0))
  (Utilities|FlowControl|Delay 0.5)
  (Actor|DestroyActor))

(fn ConstructionScript)