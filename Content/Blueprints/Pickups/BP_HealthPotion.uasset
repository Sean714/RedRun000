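; Health potion pickup built from a Paper2D sprite and a sphere trigger.
; On overlap it plays a pickup sound and Niagara effect, disables the sphere's collision and sends an UpdateHealthPotions message with a value of 1 to the overlapping actor, without filtering by type.
; A WinkOut timeline scales the sprite and offsets its height, then destroys the actor when finished.
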(event OnComponentBeginOverlap(Sphere)
  (params (OverlappedComponent :type Primitive%20Component%20Object%20Reference) (OtherActor :type Actor%20Object%20Reference) (OtherComp :type Primitive%20Component%20Object%20Reference) (OtherBodyIndex :type Integer) (bFromSweep :type Boolean) (SweepResult :type Hit%20Result%20Structure%20%28by%20ref%29))
  (bind _returnvalue (Transformation|GetActorLocation))
  ;[1 0 0] Overllap and effects
  (Audio|SpawnSoundatLocation "/Game/Assets/Sounds/Pickups/SW_Pickup1.SW_Pickup1" _returnvalue "0, 0, 0" 1.0 1.0 0.0 0 0)
  (Niagara|SpawnSystematLocation "/Game/Niagara/NS_Pickup.NS_Pickup" _returnvalue)
  (CallFunction|WinkOut)
  (Collision|SetCollisionEnabled (Variables|Default|GetSphere) "NoCollision")
  (Class|BPIUpdateStats|UpdateHealthPotions(Message) OtherActor 1))

(event Custom|WinkOut
  (bind _returnvalue (Transformation|GetActorLocation))
  (bind _papersprite (Variables|Default|GetPaperSprite))
  ;[1 0 0] WinkOut
  (bind (_direction _scale _location) (Timeline|PickupScale Play)
    (:Update
      (Transformation|SetWorldScale3D _papersprite (Math|Vector|MakeVector _scale _scale _scale))
      (Transformation|SetWorldLocation _papersprite (Math|Vector|MakeVector (.x _returnvalue) (.y _returnvalue) (+ (.z _returnvalue) (* _location 1e+02))) false false))
    (:Finished
      (Actor|DestroyActor))))

(event EventBeginPlay)

(event Collision|EventActorBeginOverlap
  (params (OtherActor :type Actor%20Object%20Reference)))

(event EventTick
  (params (DeltaSeconds :type Float%20%28single-precision%29)))

(fn ConstructionScript)