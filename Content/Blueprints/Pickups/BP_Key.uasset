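; BP_Key is a key pickup that registers itself and its linked Door in the player's key array.
; Any sphere overlap plays a sound and Niagara effect, starts WinkOut and disables collision.
; Only an overlap by the cached BP_Cornelia player adds the key and sends a collect item message.
; WinkOut uses a timeline to animate the PaperFlipbook's scale and height, then destroys the actor.
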(event OnComponentBeginOverlap(Sphere)
  (params (OverlappedComponent :type Primitive%20Component%20Object%20Reference) (OtherActor :type Actor%20Object%20Reference) (OtherComp :type Primitive%20Component%20Object%20Reference) (OtherBodyIndex :type Integer) (bFromSweep :type Boolean) (SweepResult :type Hit%20Result%20Structure%20%28by%20ref%29))
  (bind _returnvalue (Transformation|GetActorLocation))
  ;[1 0 0] Playe Sounds and Effects
  (Audio|SpawnSoundatLocation "/Game/Assets/Sounds/Pickups/SW_Pickup1.SW_Pickup1" _returnvalue "0, 0, 0" 1.0 1.0 0.0 0 0)
  (Niagara|SpawnSystematLocation "/Game/Niagara/NS_Pickup.NS_Pickup" _returnvalue)
  (CallFunction|WinkOut)
  (Collision|SetCollisionEnabled (Variables|Default|GetSphere) "NoCollision")
  ;[1 0 0] Set Key Array
  (if (== OtherActor (Variables|Default|GetPlayer))
    (Utilities|Array|Add (Variables|/Game/Blueprints/Characters/CorneliaGale/BP_Cornelia.BP_Cornelia_C|GetKeyArray (Variables|Default|GetPlayer)) (Utilities|Struct|MakeFKey self (Variables|Default|GetDoor)))
    ;[0 1 0] Collect Item
    (Class|BPIInteract|CollectItem(Message) (Variables|Default|GetPlayer) (Variables|Default|GetName) (Variables|Default|GetIcon) (Variables|Default|GetAmount))))

(event Custom|WinkOut
  (bind _returnvalue (Transformation|GetActorLocation))
  (bind _paperflipbook (Variables|Default|GetPaperFlipbook))
  ;[1 0 0] WinkOut
  (bind (_direction _scale _location) (Timeline|Timeline Play)
    (:Update
      (Transformation|SetWorldScale3D _paperflipbook (Math|Vector|MakeVector _scale _scale _scale))
      (Transformation|SetWorldLocation _paperflipbook (Math|Vector|MakeVector (.x _returnvalue) (.y _returnvalue) (+ (.z _returnvalue) (* _location 1e+02))) false false))
    (:Finished
      (Actor|DestroyActor))))

(event EventBeginPlay
  ;[1 0 0] Store Player variable
  (bind _asbp_cornelia (Utilities|Casting|CastToBP_Cornelia (Game|GetPlayerCharacter 0)))
  (Variables|Default|SetPlayer _asbp_cornelia))

(fn ConstructionScript)